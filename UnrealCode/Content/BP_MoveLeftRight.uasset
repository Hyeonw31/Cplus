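; Actor Blueprint that slides its StaticMesh back and forth along its relative X axis.
; While IsPlay is set, Tick steps the X position by a fixed amount and flips the Right flag at either end of a hard-coded range.
; Movement is per frame without delta-time scaling, so speed depends on frame rate.
; DoPlay sets IsPlay to start or stop the motion and always returns false.
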(event EventBeginPlay)

(event EventTick
  (params (DeltaSeconds :type Float%20%28single-precision%29))
  (if (Variables|Default|GetisPlay)
    (if (Variables|Default|GetRight)
      ;[1 1 1] 오른쪽으로 움직이기
      (bind _output_get (Variables|Default|SetX위치 (+ (Variables|Default|GetX위치) 1.0)))
      (Transformation|SetRelativeLocation (Variables|Default|GetStaticMesh) (Math|Vector|MakeVector _output_get 0.0 0.0) false false)
      (if (>= (Variables|Default|GetX위치) 2e+02)
        (Variables|Default|SetRight false))
      (else
        ;[1 1 1] 왼쪽으로 움직이기
        (bind _output_get_2 (Variables|Default|SetX위치 (+ (Variables|Default|GetX위치) -1.0)))
        (Transformation|SetRelativeLocation (Variables|Default|GetStaticMesh) (Math|Vector|MakeVector _output_get_2 0.0 0.0) false false)
        (if (<= (Variables|Default|GetX위치) 0.0)
          (Variables|Default|SetRight true))))))

(fn ConstructionScript)

(fn DoPlay
  (params (isPlay :type Boolean))
  (Variables|Default|SetisPlay isPlay)
  (return false))