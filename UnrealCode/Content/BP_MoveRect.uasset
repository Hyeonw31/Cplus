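; Actor Blueprint that moves its StaticMesh around a 200-unit square in the relative X-Z plane, looping indefinitely.
; Tick switches on the MoveType enum (Right, Up, Left, Down), stepping one coordinate and advancing to the next state at each corner.
; Movement is a fixed one unit per frame without delta time, so speed depends on frame rate.
; An unconnected Branch-based copy of the Left and Down logic never runs.
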(event EventBeginPlay)

(event EventTick
  (params (DeltaSeconds :type Float%20%28single-precision%29))
  (switch Utilities|FlowControl|Switch|SwitchonEN_MoveType (Variables|Default|GetMoveType)
    (:NewEnumerator0
      ;[1 1 1] 오른쪽으로 움직이기
      (bind _output_get (Variables|Default|SetX위치 (+ (Variables|Default|GetX위치) 1.0)))
      (Transformation|SetRelativeLocation (Variables|Default|GetStaticMesh) (Math|Vector|MakeVector _output_get 0.0 0.0) false false)
      (if (>= (Variables|Default|GetX위치) 2e+02)
        (Variables|Default|SetMoveType "NewEnumerator1")))
    (:NewEnumerator1
      ;[1 1 1] 위쪽으로 움직이기
      (bind _output_get_2 (Variables|Default|SetZ위치 (+ (Variables|Default|GetZ위치) 1.0)))
      (Transformation|SetRelativeLocation (Variables|Default|GetStaticMesh) (Math|Vector|MakeVector 2e+02 0.0 _output_get_2) false false)
      (if (>= (Variables|Default|GetZ위치) 2e+02)
        (Variables|Default|SetMoveType "NewEnumerator2")))
    (:NewEnumerator2
      ;[1 1 1] 왼쪽으로 움직이기
      (bind _output_get_3 (Variables|Default|SetX위치 (- (Variables|Default|GetX위치) 1.0)))
      (Transformation|SetRelativeLocation (Variables|Default|GetStaticMesh) (Math|Vector|MakeVector _output_get_3 0.0 (Variables|Default|GetZ위치)) false false)
      (if (<= (Variables|Default|GetX위치) 0.0)
        (Variables|Default|SetMoveType "NewEnumerator3")))
    (:NewEnumerator3
      ;[1 1 1] 아래쪽으로 움직이기
      (bind _output_get_4 (Variables|Default|SetZ위치 (- (Variables|Default|GetZ위치) 1.0)))
      (Transformation|SetRelativeLocation (Variables|Default|GetStaticMesh) (Math|Vector|MakeVector 0.0 0.0 _output_get_4) false false)
      (if (<= (Variables|Default|GetZ위치) 0.0)
        (Variables|Default|SetMoveType "NewEnumerator0")))))

(fn ConstructionScript)